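; BP_Chair is an interactable chair the SteveBarker player can sit on and stand up from.
; Its Box overlap shows or hides the interact HUD and binds or clears the player's Interact event.
; Sit locks movement, eases the player onto the Arrow's transform with the Rotate timeline, plays a montage, then binds Stand.
; Stand snaps to the Arrow, plays the rise montage, restores movement and clears the interaction.
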(event OnComponentBeginOverlap(Box)
  (params (OverlappedComponent :type Primitive%20Component%20Object%20Reference) (OtherActor :type Actor%20Object%20Reference) (OtherComp :type Primitive%20Component%20Object%20Reference) (OtherBodyIndex :type Integer) (bFromSweep :type Boolean) (SweepResult :type Hit%20Result%20Structure%20%28by%20ref%29))
  (bind _playerref (Variables|Default|GetPlayerRef))
  (bind _interacthud_ref (Variables|/Game/MyContents/Actors/SteveBarker.SteveBarker_C|GetInteractHUD_Ref _playerref))
  (if (== OtherActor _playerref)
    (EventDispatchers|BindEventtoInteract _playerref (delegate Custom|Sit))
    (if (UserInterface|Viewport|IsinViewport _interacthud_ref)
      (Widget|RemovefromParent _interacthud_ref))
    (UserInterface|Viewport|AddtoViewport _interacthud_ref 0)))

(event OnComponentEndOverlap(Box)
  (params (OverlappedComponent :type Primitive%20Component%20Object%20Reference) (OtherActor :type Actor%20Object%20Reference) (OtherComp :type Primitive%20Component%20Object%20Reference) (OtherBodyIndex :type Integer))
  (bind _playerref (Variables|Default|GetPlayerRef))
  (if (== OtherActor _playerref)
    (EventDispatchers|UnbindallEventsfromInteract _playerref)
    (Widget|RemovefromParent (Variables|/Game/MyContents/Actors/SteveBarker.SteveBarker_C|GetInteractHUD_Ref _playerref))))

(event Custom|Stand
  (bind _playerref (Variables|Default|GetPlayerRef))
  (bind _arrow (Variables|Default|GetArrow))
  (bind _playerref_2 (Variables|Default|GetPlayerRef))
  (bind _playerref_3 (Variables|Default|GetPlayerRef))
  (bind _playerref_4 (Variables|Default|GetPlayerRef))
  (Utilities|FlowControl|Sequence
    (:then_0
      (bind _rotate (Timeline|Rotate Stop)
        (:Update
          (Transformation|SetActorLocationAndRotation _playerref (Math|Vector|Lerp(Vector) (Transformation|GetActorLocation _playerref_2) (Transformation|GetWorldLocation _arrow) _rotate) (Math|Rotator|Lerp(Rotator) (Transformation|GetActorRotation _playerref_2) (Transformation|GetWorldRotation _arrow) _rotate)))
        (:Finished
          (Animation|PlayAnimMontage _playerref "/Game/MyContents/Actors/Animation/Montage/Stand_To_Sit_Montage.Stand_To_Sit_Montage" 1.0 "None")
          (EventDispatchers|BindEventtoInteract (Variables|Default|GetPlayerRef) (delegate Custom|Stand)))))
    (:then_1
      (EventDispatchers|UnbindEventfromInteract _playerref_4 (delegate Custom|Sit))
      (Transformation|SetActorLocation _playerref_4 (Transformation|GetWorldLocation (Variables|Default|GetArrow)) false false)
      (Animation|PlayAnimMontage (Variables|Default|GetPlayerRef) "/Game/MyContents/Actors/Animation/Montage/sit_to_stand__with_root_Montage.sit_to_stand__with_root_Montage" 1.0 "None")
      (Utilities|FlowControl|Delay 0.2)
      (Variables|/Game/MyContents/Actors/SteveBarker.SteveBarker_C|SetCanMove _playerref_3 true)
      (Widget|RemovefromParent (Variables|/Game/MyContents/Actors/SteveBarker.SteveBarker_C|GetInteractHUD_Ref _playerref_3))
      (EventDispatchers|UnbindallEventsfromInteract _playerref_3))))

(event Custom|Sit
  (bind _playerref (Variables|Default|GetPlayerRef))
  (bind _arrow (Variables|Default|GetArrow))
  (bind _playerref_2 (Variables|Default|GetPlayerRef))
  (Variables|/Game/MyContents/Actors/SteveBarker.SteveBarker_C|SetCanMove (Variables|Default|GetPlayerRef) false)
  (bind _rotate (Timeline|Rotate PlayFromStart)
    (:Update
      (Transformation|SetActorLocationAndRotation _playerref (Math|Vector|Lerp(Vector) (Transformation|GetActorLocation _playerref_2) (Transformation|GetWorldLocation _arrow) _rotate) (Math|Rotator|Lerp(Rotator) (Transformation|GetActorRotation _playerref_2) (Transformation|GetWorldRotation _arrow) _rotate)))
    (:Finished
      (Animation|PlayAnimMontage _playerref "/Game/MyContents/Actors/Animation/Montage/Stand_To_Sit_Montage.Stand_To_Sit_Montage" 1.0 "None")
      (EventDispatchers|BindEventtoInteract (Variables|Default|GetPlayerRef) (delegate Custom|Stand)))))

(event EventBeginPlay
  (bind _assteve_barker (Utilities|Casting|CastToSteveBarker (Game|Player|GetPlayerPawn 0)))
  (Variables|Default|SetPlayerRef _assteve_barker))

(fn ConstructionScript)